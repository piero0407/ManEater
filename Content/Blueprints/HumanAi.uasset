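; HumanAi is the AI controller for human NPCs that detect and react to the player character.
; It runs the HumanBehaviour tree on BeginPlay and routes perception updates to HandleSense by the sense class's display name.
; Only sight of a ThirdPersonCharacter is handled: it sets IsInvestigating to the sensed state.
; On a successful sighting it also plays a chase sound and stores the character as TargetLocationActor on the blackboard.
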(event `self.ReceiveBeginPlay`
  (`self.RunBehaviorTree` "/Game/Blueprints/HumanBehaviour.HumanBehaviour"))

(event `self.AIPerception.OnTargetPerceptionUpdated`
  (params (Actor :type "Actor Object Reference") (Stimulus :type "AIStimulus Structure"))
  (bind _returnvalue (`AIPerceptionSystem.GetSenseClassForStimulus` Stimulus))
  (`self.HandleSense` (`KismetSystemLibrary.GetClassDisplayName` _returnvalue) Stimulus Actor))

(fn `HandleSense`
  (params (Selection :type String) (Stimulus :type "AIStimulus Structure") (`Sense Actor` :type "Actor Object Reference"))
  (bind (_stimulus_age _stimulus_expirationage _stimulus_strength _stimulus_stimuluslocation _stimulus_receiverlocation _stimulus_tag _stimulus_bsuccessfullysensed) (break `AIStimulus` (`local.Stimulus`)))
  (cast `/Game/Blueprints/ThirdPersonCharacter` `Sense Actor`)
  (switch `string` Selection
    (:`AiSense_Sight`
      (`BlackboardComponent.SetValueAsBool` (`self.Blackboard`) "IsInvestigating" _stimulus_bsuccessfullysensed)
      (if _stimulus_bsuccessfullysensed
        (`GameplayStatics.SpawnSound2D` "/Game/SFX/sfx_persecucion_v1.sfx_persecucion_v1" 1.0 1.0 0.0 null)
        (`BlackboardComponent.SetValueAsObject` (`self.Blackboard`) "TargetLocationActor" (`local.Sense Actor`))))))

(fn `UserConstructionScript`)